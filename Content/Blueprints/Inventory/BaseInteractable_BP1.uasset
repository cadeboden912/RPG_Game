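; BaseInteractable_BP1 is an interactable pickup actor that gives the player an inventory item.
; Its construction script looks up ItemInfo from the ItemInfo_DT data table, using the ItemName enum converted to a row name.
; On Interact, it passes that info to PlayerCharacter_BP's PickupItem and then destroys itself.
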(event EventInteract
  (bind _asplayer_character_bp (Utilities|Casting|CastToPlayerCharacter_BP (Game|GetPlayerCharacter 0)))
  (Default|PickupItem _asplayer_character_bp (Variables|Default|GetItemInfo))
  (Actor|DestroyActor))

(fn ConstructionScript
  (bind _returnvalue (Utilities|GetDataTableRow "/Game/Blueprints/Inventory/DataTables/ItemInfo_DT.ItemInfo_DT" (Utilities|String|StringToName (Utilities|String|EnumtoString (Variables|Default|GetItemName))))
    (:then
      (Variables|Default|SetItemInfo _returnvalue))))